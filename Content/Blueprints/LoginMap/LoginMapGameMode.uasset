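; Game mode for the login map that puts the login screen in front of the player when play begins.
; BeginPlay calls ShowLoginWidget, which creates the Login_WD widget for the first player controller if no valid reference exists and caches it.
; The widget is added to the viewport unless already shown, and input switches to Game and UI without hiding the cursor during capture.
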(event `self.ReceiveBeginPlay`
  (`self.ShowLoginWidget`))

(fn `ShowLoginWidget`
  (`/Engine/EditorBlueprintResources/StandardMacros.IsValid` (`self.LoginWidgetRef`)
    (:`Is Valid`
      (if (not (`Widget.IsInViewport` (`self.LoginWidgetRef`)))
        (`UserWidget.AddToViewport` (`self.LoginWidgetRef`) 0 :!label _label)
        (`WidgetBlueprintLibrary.SetInputMode_GameAndUIEx` (`GameplayStatics.GetPlayerController` 0) null "DoNotLock" false)))
    (:`Is Not Valid`
      (bind _returnvalue (`|CreateWidget` "/Game/UMG/LoginMap/Login_WD.Login_WD_C" (`GameplayStatics.GetPlayerController` 0)))
      (set `self.LoginWidgetRef` _returnvalue)
      (goto _label))))

(fn `UserConstructionScript`)